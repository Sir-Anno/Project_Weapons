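; Base weapon Blueprint for projectile weapons that spawns a projectile actor each time it fires.
; FireWeapon runs the parent logic, then spawns the magazine's ammo type at the FirePoint, always spawning regardless of collision.
; Shot direction is randomized within a cone around the FirePoint's forward vector, with the Accuracy value as the half-angle in degrees.
; The FireProjectile function is an empty stub.
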(fn `Fire weapon`
  (bind _firepoint (`self.FirePoint`))
  (`parent.Fire weapon`)
  (`|SpawnActorFromClass` (`/Game/Blueprints/Weapons/Ammo/BP_MagazineBase.Ammo type` (`self.Magazine`)) (`KismetMathLibrary.MakeTransform` (`SceneComponent.K2_GetComponentLocation` _firepoint) (`KismetMathLibrary.MakeRotFromX` (`KismetMathLibrary.RandomUnitVectorInConeInDegrees` (`SceneComponent.GetForwardVector` _firepoint) (`self.Accuracy`)))) "AlwaysSpawn" "SelectDefaultAtRuntime" null null))

(fn `FireProjectile`)

(fn `UserConstructionScript`
  (`parent.UserConstructionScript`))