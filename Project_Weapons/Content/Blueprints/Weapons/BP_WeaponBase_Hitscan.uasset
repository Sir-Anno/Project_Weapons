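; BP_WeaponBase_Hitscan is a hitscan weapon Blueprint that extends its parent's FireWeapon with an instant line trace.
; FireWeapon traces from FirePoint over WeaponRange, applies Damage to the hit actor and attaches a temporary laser-hit decal aligned to the impact normal.
; The random-cone direction has a zero angle, so shots have no spread, and traces draw debug lines.
; A separate FireHitScan function only performs a fixed-length debug trace.
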(fn `Fire weapon`
  (bind _returnvalue (`SceneComponent.K2_GetComponentLocation` (`self.FirePoint`)))
  (`parent.Fire weapon`)
  (bind _outhit (`KismetSystemLibrary.LineTraceSingle` :`Start` _returnvalue :`End` (+ _returnvalue (* (`KismetMathLibrary.RandomUnitVectorInConeInDegrees` (`SceneComponent.GetForwardVector` (`self.FirePoint`))) (`self.Weapon range`))) :`TraceChannel` "TraceTypeQuery1" :`DrawDebugType` "ForDuration" :`DrawTime` 1.0))
  (bind (_bblockinghit _binitialoverlap _time _distance _location _impactpoint _normal _impactnormal _physmat _hitactor _hitcomponent) (`GameplayStatics.BreakHitResult` _outhit))
  (`GameplayStatics.ApplyDamage` _hitactor (`self.Damage`))
  (`GameplayStatics.SpawnDecalAttached` "/Game/Assets/Materials/M_LaserHitDecal.M_LaserHitDecal" (64.0 64.0 64.0) _hitcomponent "None" _location (`KismetMathLibrary.Conv_VectorToRotator` _impactnormal) "KeepWorldPosition" 10.0))

(fn `FireHitScan`
  (bind _firepoint (`self.FirePoint`))
  (bind _returnvalue (`SceneComponent.K2_GetComponentLocation` _firepoint))
  (`KismetSystemLibrary.LineTraceSingle` :`Start` _returnvalue :`End` (+ _returnvalue (* (`SceneComponent.GetForwardVector` _firepoint) 10000.0)) :`TraceChannel` "TraceTypeQuery1" :`DrawDebugType` "ForDuration" :`DrawTime` 0.5))

(fn `UserConstructionScript`
  (`parent.UserConstructionScript`))