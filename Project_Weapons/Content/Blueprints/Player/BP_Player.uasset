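; BP_Player is the player Blueprint that handles weapon equipping, firing and a magazine count.
; On BeginPlay it binds events to the player controller's fire and cease-fire dispatchers, which drive the weapon's trigger state.
; EquipWeapon swaps a child actor's class, rebuilds the weapon HUD and broadcasts an equip dispatcher.
; Helper functions add and remove magazines, with additions also broadcast through a dispatcher.
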(event `self.ReceiveBeginPlay`
  (bind _asbp_player_controller (cast `/Game/Blueprints/Player/BP_PlayerController` (`GameplayStatics.GetPlayerController` 0)))
  (add `/Game/Blueprints/Player/BP_PlayerController.ED_Fire` _asbp_player_controller (`|CreateDelegate` :!event `Fire weapon`))
  (add `/Game/Blueprints/Player/BP_PlayerController.ED_CeaseFire` _asbp_player_controller (`|CreateDelegate` :!event `Cease fire`)))

(event `Fire weapon`
  (bind _weapon (`self.Weapon`)
    (:`then`
      (set `/Game/Blueprints/Weapons/BP_WeaponBase.Trigger down` true _weapon)
      (`/Game/Blueprints/Weapons/BP_WeaponBase.Pull trigger` _weapon))
    (:`else`)))

(event `Cease fire`
  (bind _weapon (`self.Weapon`)
    (:`then`
      (set `/Game/Blueprints/Weapons/BP_WeaponBase.Trigger down` false _weapon))
    (:`else`)))

(fn `AddMagazineToInventory`
  (bind _result (`/Engine/EditorBlueprintResources/StandardMacros.IncrementInt` (`self.MagazineCount`))
    (:`  `
      (`self.ED_AddMagazineToInventory` _result))))

(fn `EquipWeapon`
  (params (Weapon :type "Actor Class Reference"))
  (`ChildActorComponent.SetChildActorClass` (`self.EquipedWeapon`) Weapon)
  (bind _asbp_weapon_base (cast `/Game/Blueprints/Weapons/BP_WeaponBase` (`ChildActorComponent.ChildActor` (`self.EquipedWeapon`))))
  (set `self.Weapon` _asbp_weapon_base)
  (bind _foundwidgets (`WidgetBlueprintLibrary.GetAllWidgetsOfClass` "/Game/Blueprints/Player/BPW_WeaponHUD.BPW_WeaponHUD_C"))
  (for _array_element _foundwidgets
    (`Widget.RemoveFromParent` _array_element))
  (bind _returnvalue (`|CreateWidget` "/Game/Blueprints/Player/BPW_WeaponHUD.BPW_WeaponHUD_C"))
  (`UserWidget.AddToViewport` _returnvalue 0)
  (`self.ED_EquipWeapon`))

(fn `RemoveMagazineFromInventory`
  (bind _result (`/Engine/EditorBlueprintResources/StandardMacros.DecrementInt` (`self.MagazineCount`))
    (:`  `
      (set `self.MagazineCount` _result))))

(fn `UserConstructionScript`)