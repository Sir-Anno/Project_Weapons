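; Player controller Blueprint that turns Enhanced Input actions into player pawn movement, look, jump and fire signals.
; BeginPlay adds the input mapping context, then move and look actions drive movement along the pawn's axes and controller yaw/pitch.
; Fire press and release call the Fire and CeaseFire event dispatchers rather than acting on the pawn directly.
; Jump casts the controlled pawn to BP_Player before calling Jump.
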(event `self.ReceiveBeginPlay`
  (`EnhancedInputSubsystemInterface.AddMappingContext` (subsystem `EnhancedInputLocalPlayerSubsystem`) "/Game/Input/IMC_Input.IMC_Input" 0 (struct)))

(event `EnhancedInput|/Game/Input/IA_Movement`
  (params (ActionValue :type "Vector2D Structure") (ElapsedSeconds :type "Float (double-precision)") (TriggeredSeconds :type "Float (double-precision)") (InputAction :type "InputAction Object Reference" :default "/Game/Input/IA_Movement.IA_Movement"))
  (bind _returnvalue (`self.K2_GetPawn`))
  (bind _returnvalue_2 (`self.K2_GetPawn`))
  (:`Triggered`
    (`Pawn.AddMovementInput` _returnvalue (`self.GetActorRightVector` _returnvalue) ActionValue_X false)
    (`Pawn.AddMovementInput` _returnvalue_2 (`self.GetActorForwardVector` _returnvalue_2) ActionValue_Y false)))

(event `EnhancedInput|/Game/Input/IA_Look`
  (params (ActionValue :type "Vector2D Structure") (ElapsedSeconds :type "Float (double-precision)") (TriggeredSeconds :type "Float (double-precision)") (InputAction :type "InputAction Object Reference" :default "/Game/Input/IA_Look.IA_Look"))
  (:`Triggered`
    (`Pawn.AddControllerYawInput` (`self.K2_GetPawn`) ActionValue_X)
    (`Pawn.AddControllerPitchInput` (`self.K2_GetPawn`) ActionValue_Y)))

(event `EnhancedInput|/Game/Input/IA_Fire`
  (params (ActionValue :type Boolean) (ElapsedSeconds :type "Float (double-precision)") (TriggeredSeconds :type "Float (double-precision)") (InputAction :type "InputAction Object Reference" :default "/Game/Input/IA_Fire.IA_Fire"))
  (:`Started`
    (`self.ED_Fire`))
  (:`Completed`
    (`self.ED_CeaseFire`)))

(event `EnhancedInput|/Game/Input/IA_Jump`
  (params (ActionValue :type Boolean) (ElapsedSeconds :type "Float (double-precision)") (TriggeredSeconds :type "Float (double-precision)") (InputAction :type "InputAction Object Reference" :default "/Game/Input/IA_Jump.IA_Jump"))
  (:`Triggered`
    (bind _asbp_player (cast `/Game/Blueprints/Player/BP_Player` (`self.K2_GetPawn`)))
    (`Character.Jump` _asbp_player)))

(fn `UserConstructionScript`)