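; BP_ItemPickup is a world pickup that gives BP_Player a weapon or a magazine on overlap.
; Its construction script sets the Magazine child actor to the configured Item class.
; On overlap, EquipSlot selects between equipping Item as a weapon and adding a magazine to the inventory.
; The actor then hides and reappears after a fixed delay, with its collision left untouched.
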(event `self.PickupCollision.OnComponentBeginOverlap`
  (params (OverlappedComponent :type "PrimitiveComponent Object Reference") (OtherActor :type "Actor Object Reference") (OtherComp :type "PrimitiveComponent Object Reference") (OtherBodyIndex :type Integer) (bFromSweep :type Boolean) (SweepResult :type "HitResult Structure (by ref)"))
  (bind _asbp_player (cast `/Game/Blueprints/Player/BP_Player` OtherActor))
  (set `self.As BP Player` _asbp_player)
  (switch `/Game/Blueprints/E_EquiptSlots` (`self.Equip slot`)
    (:`NewEnumerator0`
      (`/Game/Blueprints/Player/BP_Player.EquipWeapon` (`self.As BP Player`) (`self.Item`)))
    (:`NewEnumerator1`
      (`/Game/Blueprints/Player/BP_Player.AddMagazineToInventory` (`self.As BP Player`))))
  (`self.SetActorHiddenInGame` true)
  (`KismetSystemLibrary.Delay` 5.0)
  (`self.SetActorHiddenInGame` false))

(fn `UserConstructionScript`
  (`ChildActorComponent.SetChildActorClass` (`self.Magazine`) (`self.Item`)))